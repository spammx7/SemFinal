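; Enemy character Blueprint that chases the player once it spots a pawn and triggers an attack animation.
; PawnSensing sets a seen flag on any detected pawn and calls the follow event, which runs AI MoveTo toward player character 0.
; The move node's Then output plays a montage if attacking is allowed, clearing that flag, which this graph never resets.
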(event `self.PawnSensing.OnSeePawn`
  (params (Pawn :type "Pawn Object Reference"))
  (set `self.itseespawn` true)
  (`self.followplayer`))

(event `followplayer`
  (if (`self.itseespawn`)
    (`|AIMoveTo` self (0.0 0.0 0.0) (`GameplayStatics.GetPlayerCharacter` 0)
      (:`then`
        (if (`self.canattack?`)
          (set `self.canattack?` false)
          (`self.PlayAnimMontage` null))))))

(fn `UserConstructionScript`)